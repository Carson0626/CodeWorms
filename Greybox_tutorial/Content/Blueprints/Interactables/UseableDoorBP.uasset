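; Interactable door Blueprint that alternates between opening and closing each time UseInteract fires.
; A FlipFlop plays or reverses the OpenDoor timeline, whose track is added to the cached actor yaw to set the StaticMesh's relative rotation.
; The construction script caches that rotation in NewVar0 and computes an OpenRotation that the graph never reads.
; Collision-toggling nodes are present but never run.
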(event EventUseInteract
  (params (UsingActor :type Actor%20Object%20Reference))
  (Utilities|FlowControl|FlipFlop
    (:A
      (bind _newtrack_0 (Timeline|OpenDoor Play)
        (:Update
          (Transformation|SetRelativeRotation (Variables|Default|GetStaticMesh) (Math|Rotator|MakeRotator 0.0 0.0 (+ _newtrack_0 (.Yaw (Math|Rotator|BreakRotator (Variables|Default|GetNewVar_0))))) false false))))
    (:B
      (Timeline|OpenDoor Reverse))))

(fn ConstructionScript
  (bind _returnvalue (Transformation|GetActorRotation))
  (bind (_roll _pitch _yaw) (Math|Rotator|BreakRotator _returnvalue))
  (Variables|Default|SetOpenRotation (Math|Rotator|MakeRotator _roll _pitch (+ _yaw 9e+01)))
  (Variables|Default|SetNewVar_0 _returnvalue))