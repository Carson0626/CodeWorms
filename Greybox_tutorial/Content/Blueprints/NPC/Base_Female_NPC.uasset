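; Base female NPC Blueprint that builds a customizable character appearance from mesh and material variables.
; The construction script assigns skeletal meshes to top, bottom and shoe components and slaves them to the body Mesh via master pose, so they share its animation.
; Hair is a swappable static mesh, and per-part material variables set clothing, hair and skin looks.
; BeginPlay has no logic.
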(event EventBeginPlay)

(fn ConstructionScript
  (Class|SkinnedMeshComponent|SetSkeletalMesh (Variables|Default|GetBOTTOM) (Variables|Default|GetBottomVar) true)
  (Class|SkinnedMeshComponent|SetSkeletalMesh (Variables|Default|GetTOP) (Variables|Default|GetTopVar) true)
  (Class|SkinnedMeshComponent|SetSkeletalMesh (Variables|Default|GetSHOES) (Variables|Default|GetShoeVar) true)
  (Class|SkinnedMeshComponent|SetMasterPoseComponent (Variables|Default|GetTOP) (Variables|Character|GetMesh) false)
  (Components|StaticMesh|SetStaticMesh (Variables|Default|GetHAIR) (Variables|Default|GetHairVar))
  (Rendering|Material|SetMaterial (Variables|Default|GetBOTTOM) 0 (Variables|Default|GetBottomColor))
  (Rendering|Material|SetMaterial (Variables|Default|GetTOP) 0 (Variables|Default|GetTopColor))
  (Rendering|Material|SetMaterial (Variables|Default|GetSHOES) 0 (Variables|Default|GetShoeColor))
  (Rendering|Material|SetMaterial (Variables|Default|GetHAIR) 0 (Variables|Default|GetHairColor))
  (Rendering|Material|SetMaterial (Variables|Character|GetMesh) 0 (Variables|Default|GetSkinVar)))