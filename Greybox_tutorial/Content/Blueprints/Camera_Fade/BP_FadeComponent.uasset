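; BP_FadeComponent is a component that fades its owning StaticMeshActor out and back in when ToggleHideMesh is called.
; BeginPlay caches the slot 0 material, which must be a base Material, and creates a dynamic instance of FadeMaterial.
; Hiding swaps in that instance, and Tick drives its Fade parameter through FadeCurve at FadeRate.
; Once fully visible again, Tick restores the original material.
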(event EventBeginPlay
  ;[1 1 1] Setup Component
  (bind _asstatic_mesh_actor (Utilities|Casting|CastToStaticMeshActor (Components|GetOwner))) ; Get Static Mesh Actor
  (bind _output_get (Variables|Default|SetParrentMesh _asstatic_mesh_actor))
  (bind _asmaterial (Utilities|Casting|CastToMaterial (Rendering|Material|GetMaterial (Variables|/Script/Engine.StaticMeshActor|GetStaticMeshComponent _output_get) 0)))
  (Variables|Default|SetBaseMaterial _asmaterial)
  (bind _returnvalue (Rendering|Material|CreateDynamicMaterialInstance (Variables|Default|GetFadeMaterial) "None" :!class /Script/Engine.KismetMaterialLibrary))
  (Variables|Default|SetFadeMaterialMID _returnvalue))

(event EventTick
  (params (DeltaSeconds :type Float%20%28single-precision%29))
  ;[1 1 1] Fade over time
  (Variables|Default|SetDeltaTime DeltaSeconds)
  (Utilities|IsValid (Variables|Default|GetParrentMesh)
    (:Is%20Valid
      (if (Variables|Default|GetHidden) ; Hidden?
        (Variables|Default|SetCurrentFade (Math|Float|Clamp(Float) (- (Variables|Default|GetCurrentFade) (* (Variables|Default|GetDeltaTime) (Variables|Default|GetFadeRate)))))
        (else
          (Variables|Default|SetCurrentFade (Math|Float|Clamp(Float) (+ (Variables|Default|GetCurrentFade) (* (Variables|Default|GetDeltaTime) (Variables|Default|GetFadeRate)))))))
      (Rendering|Material|SetScalarParameterValue (Variables|Default|GetFadeMaterialMID) "Fade" (Math|Curves|GetFloatValue (Variables|Default|GetFadeCurve) (Variables|Default|GetCurrentFade)) :!class /Script/Engine.MaterialInstanceDynamic)
      (if (and (== (Variables|Default|GetCurrentFade) 1.0) (not (Variables|Default|GetHidden)))
        (Rendering|Material|SetMaterial (Variables|/Script/Engine.StaticMeshActor|GetStaticMeshComponent (Variables|Default|GetParrentMesh)) 0 (Variables|Default|GetBaseMaterial))))))

(fn ToggleHideMesh
  (params (Hidden :type Boolean))
  ;[1 1 1] Toggle hidden / show
  (if (Math|Boolean|NotEqual(Boolean) Hidden (Variables|Default|GetHidden)) ; Only if Changing
    (bind _output_get (Variables|Default|SetHidden Hidden))
    (if _output_get ; True = Hidden
      (Rendering|Material|SetMaterial (Variables|/Script/Engine.StaticMeshActor|GetStaticMeshComponent (Variables|Default|GetParrentMesh)) 0 (Variables|Default|GetFadeMaterialMID)))))