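; Behavior tree decorator that passes when the AI currently sees the player and the player is eating.
; It reads sight-perceived actors from the AI controller's perception component and compares them with the blackboard's PlayerKey object.
; The loop returns false on the first non-matching actor, so only the first perceived actor is effectively tested.
; On a match, it casts the player object and checks its IsEating flag.
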(fn PerformConditionCheckAI
  (params (OwnerController :type AI%20Controller%20Object%20Reference) (ControlledPawn :type Pawn%20Object%20Reference))
  (bind _returnvalue (AI|GetBlackboard ControlledPawn))
  (bind _player_key (LocalVariables|GetPlayer_Key))
  (bind _returnvalue_2 (AI|Components|Blackboard|GetValueasObject _returnvalue _player_key))
  (bind _array_element (Utilities|Array|ForEachLoopwithBreak (Class|AIPerceptionComponent|GetCurrentlyPerceivedActors (Class|AIController|GetAIPerceptionComponent (AI|GetAIController ControlledPawn)) "/Script/AIModule.AISense_Sight") :!label _label)
    (:LoopBody
      (if (== _array_element _returnvalue_2) ; is player visible?
        (goto _label Break)
        (else
          _)))
    (:Completed
      (if (and (== _array_element _returnvalue_2) (Variables|/Game/Player+AI/Blueprints/_00._00_C|GetisEating? (.As%2000 (Utilities|Casting|CastTo_00 _returnvalue_2)))) ; if player is visible and eating
        (return true)
        (else
          _))))
  (return false))