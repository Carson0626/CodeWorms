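; OwnerAI is the AI logic for an owner character, driving blackboard values that include a dog-punishment flag.
; On BeginPlay it resets the iterator blackboard key to zero.
; Each received cat call toggles a FlipFlop and writes the result to the PunishDog key.
; Tick is empty, and the tagged point-of-interest gathering and player-distance debug print are disconnected.
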(event Custom|EventRecieveCatCall
  (bind _isa (Utilities|FlowControl|FlipFlop)
    (:A
      _)
    (:B
      _))
  (AI|Components|Blackboard|SetValueasBool (AI|GetBlackboard 0) (Variables|Default|GetPunishDog) _isa))

(event EventBeginPlay
  (Class|BlackboardComponent|SetValueasInt (AI|GetBlackboard 0) (Variables|Default|GetIteratorKey)))

(event EventTick
  (params (DeltaSeconds :type Float%20%28single-precision%29)))

(fn ConstructionScript
  (|CallParentFunction))